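; BP_CharacterActorInventory is a base Blueprint, named as a character inventory actor, that provides visual cues for interaction and pointing.
; Enter and exit interact events show and hide its TextRender.
; Separate appear and disappear events, named as subsystem calls, show and hide the ArrowPointing component.
; The graph only toggles visibility, without propagating to children, and holds no inventory logic; the construction script is empty.
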(event EventOnSubsystemCallAppear
  (Rendering|SetVisibility (Variables|Default|GetArrowPointing) true false))

(event EventOnSubsystemCallDisappear
  (Rendering|SetVisibility (Variables|Default|GetArrowPointing) false false))

(event EventOnEnterInteract
  (Rendering|SetVisibility (Variables|Default|GetTextRender) true false))

(event EventOnExitInteract
  (Rendering|SetVisibility (Variables|Default|GetTextRender) false false))

(fn ConstructionScript)