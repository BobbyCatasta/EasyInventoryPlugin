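; Player character Blueprint that handles Enhanced Input movement and look, plus finding and trading with inventory actors.
; Each tick, a short forward sphere trace holds one ActorWithInventory as target until no such actor is hit, notifying it on enter and exit.
; Interact opens an InventorySubsystem trade session between both storages and shows WB_ItemWindow in UI-only mode with a cursor.
; Scan asks the same subsystem to show actor positions.
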(event Input|EnhancedActionEvents|EnhancedInputActionIA_Interact
  (params (ActionValue :type Boolean) (ElapsedSeconds :type Float%20%28double-precision%29) (TriggeredSeconds :type Float%20%28double-precision%29) (InputAction :type Input%20Action%20Object%20Reference :default "/EasyInventoryPlugin/ThirdPerson/Input/Actions/IA_Interact.IA_Interact"))
  (CallFunction|CreateTrade))

(event EventBeginPlay
  (|CallParentFunction)
  (Input|AddMappingContext (PlayerController|LocalPlayerSubsystems|GetEnhancedInputLocalPlayerSubsystem (Game|GetPlayerController 0)) "/EasyInventoryPlugin/ThirdPerson/Input/IMC_Default.IMC_Default" 0 "(bIgnoreAllPressedKeysUntilRelease=True,bForceImmediately=False,bNotifyUserSettings=False)"))

(event Collision|EventActorBeginOverlap
  (params (OtherActor :type Actor%20Object%20Reference))
  (|CallParentFunction OtherActor))

(event EventTick
  (params (DeltaSeconds :type Float%20%28single-precision%29))
  (|CallParentFunction DeltaSeconds)
  (CallFunction|CheckInventory))

(event Input|EnhancedActionEvents|EnhancedInputActionIA_Move
  (params (ActionValue :type Vector%202D%20Structure) (ElapsedSeconds :type Float%20%28double-precision%29) (TriggeredSeconds :type Float%20%28double-precision%29) (InputAction :type Input%20Action%20Object%20Reference :default "/EasyInventoryPlugin/ThirdPerson/Input/Actions/IA_Move.IA_Move"))
  (bind _returnvalue (Game|GetPlayerController 0))
  (bind _returnvalue_2 (Pawn|GetControlRotation _returnvalue :!class /Script/Engine.Controller))
  (bind _returnvalue_3 (Math|Rotator|MakeRotator 0.0 0.0 (.yaw _returnvalue_2)))
  (Pawn|Input|AddMovementInput (Math|Vector|GetForwardVector _returnvalue_3) (.y ActionValue) false)
  (Pawn|Input|AddMovementInput (Math|Vector|GetRightVector _returnvalue_3) (.x ActionValue) false))

(event Input|EnhancedActionEvents|EnhancedInputActionIA_Look
  (params (ActionValue :type Vector%202D%20Structure) (ElapsedSeconds :type Float%20%28double-precision%29) (TriggeredSeconds :type Float%20%28double-precision%29) (InputAction :type Input%20Action%20Object%20Reference :default "/EasyInventoryPlugin/ThirdPerson/Input/Actions/IA_Look.IA_Look"))
  (Pawn|Input|AddControllerYawInput (.x ActionValue))
  (Pawn|Input|AddControllerPitchInput (.y ActionValue)))

(event Input|EnhancedActionEvents|EnhancedInputActionIA_Scan
  (params (ActionValue :type Boolean) (ElapsedSeconds :type Float%20%28double-precision%29) (TriggeredSeconds :type Float%20%28double-precision%29) (InputAction :type Input%20Action%20Object%20Reference :default "/EasyInventoryPlugin/ThirdPerson/Input/Actions/IA_Scan.IA_Scan"))
  (Class|InventorySubsystem|ShowPositionActors (Subsystems|GetInventorySubsystem)))

(fn ConstructionScript)

(fn CheckInventory
  (bind _outhit (Collision|SphereTraceForObjects (Transformation|GetActorLocation) (+ (Transformation|GetActorLocation) (* (Transformation|GetActorForwardVector) 5e+01)) 56.0 (LocalVariables|Getelements) false 0 "None"))
  (bind _asactor_with_inventory (Utilities|Casting|CastToActorWithInventory (.hitactor _outhit))
    (:then
      (if (not (Utilities|IsValid (Variables|Default|GetotherInventoryActor)))
        (Variables|Default|SetotherInventoryActor _asactor_with_inventory)
        (Class|ActorwithInventory|OnEnterInteract (Variables|Default|GetotherInventoryActor))))
    (:CastFailed
      (if (Utilities|IsValid (Variables|Default|GetotherInventoryActor))
        (Class|ActorwithInventory|OnExitInteract (Variables|Default|GetotherInventoryActor))
        (Variables|Default|SetotherInventoryActor 0)))))

(fn CreateTrade
  (bind _returnvalue (Game|GetPlayerController 0))
  (if (and (not (Utilities|IsValid (Class|InventorySubsystem|GetCurrentTradingSession (Subsystems|GetInventorySubsystem)))) (Utilities|IsValid (Variables|Default|GetotherInventoryActor)))
    (Class|InventorySubsystem|GenerateTradeSession (Subsystems|GetInventorySubsystem) (Variables|Default|GetInventoryStorage) (Variables|/Script/EasyInventoryPlugin.ActorWithInventory|GetItemStorageComponent (Variables|Default|GetotherInventoryActor)))
    (bind _output_get (LocalVariables|SetplayerController _returnvalue))
    (bind _returnvalue_2 (UserInterface|CreateWidget "/EasyInventoryPlugin/PlaceholderWidgets/WB_ItemWindow.WB_ItemWindow_C" _output_get))
    (UserInterface|Viewport|AddtoViewport _returnvalue_2 0)
    (Default|InitializeWidget _returnvalue_2)
    (Input|SetInputModeUIOnly _returnvalue _returnvalue_2 "DoNotLock" false)
    (Variables|/Script/Engine.PlayerController|SetbShowMouseCursor _returnvalue true)))