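; BP_WinChecker is a trigger actor that tells the player whether their inventory holds the required items.
; On overlap with a CBP_PlayerInventory actor, it reveals a text render and asks the InventorySubsystem to compare that actor's InventoryStorage against ItemsRequired.
; The text shows an Italian success or failure message; no other win logic runs.
; Any end overlap hides the text, without checking which actor left.
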(event Collision|EventActorBeginOverlap
  (params (OtherActor :type Actor%20Object%20Reference))
  (bind _ascbp_player_inventory (Utilities|Casting|CastToCBP_PlayerInventory OtherActor))
  (Rendering|SetVisibility (Variables|Default|GetTextRender) true false)
  (bind _returnvalue (Class|InventorySubsystem|HasActorwithInventoryRightItems (Subsystems|GetInventorySubsystem) (Variables|/EasyInventoryPlugin/Blueprints/CBP_PlayerInventory.CBP_PlayerInventory_C|GetInventoryStorage _ascbp_player_inventory) (Variables|Default|GetitemsRequired)))
  (if _returnvalue
    (Rendering|Components|TextRender|SetText (Variables|Default|GetTextRender) (Utilities|Text|ToText(String) "Hai gli item corretti!"))
    (else
      (Rendering|Components|TextRender|SetText (Variables|Default|GetTextRender) (Utilities|Text|ToText(String) "Non hai gli Item Corretti")))))

(event Collision|EventActorEndOverlap
  (params (OtherActor :type Actor%20Object%20Reference))
  (Rendering|SetVisibility (Variables|Default|GetTextRender) false false))

(fn ConstructionScript)